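; A 2D flipbook demon enemy that patrols target points, chases the player and attacks up close.
; It stays dormant until flagged and the player is within range, then appears with particles and sound.
; Tick then drives state-flag animation, targeting, X-axis movement and timed attacks that stop it and subtract player health after a delay.
; Bullet overlaps cause hurt or death, and death launches a health pickup toward the player.
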(event Custom|Spawn
  (if (<= (Transformation|GetDistanceTo (Game|Player|GetPlayerPawn 0)) (Variables|Default|GetSpawnDistance))
    (Utilities|FlowControl|DoOnce false
      (:Completed
        (Components|Activation|Activate (Variables|Default|GetParticleSystem) false)
        (Utilities|FlowControl|Delay 0.8)
        (Components|Activation|Activate (Variables|Default|GetSpawnAudio) false)
        (Rendering|SetVisibility (Variables|Default|GetSprite) true false)
        (Utilities|FlowControl|Delay 1.6)
        (Components|DestroyComponent (Variables|Default|GetParticleSystem))
        (Variables|Default|SetbisSpawned true)
        (Components|Activation|Activate (Variables|Default|GetMonster) false)
        (Variables|/Script/Engine.PrimitiveComponent|SetbGenerateOverlapEvents (Variables|Collision|GetCapsuleComponent) true)))))

(event Custom|ShoudSpaawn
  (Variables|Default|SetSpawnDistance 1e+05)
  (Variables|Default|SetbisShoudSpawn true))

(event Custom|UpdateAnimation
  ;[1 1 1] Handle Animation
  (Sprite|SetFlipbook (Variables|Default|GetSprite) (select (Variables|Default|GetbisDead) "/Game/DemonSlayer/Textures/Enemy/Demon1/Death/DemonDeath.DemonDeath" (select (Variables|Default|GetbisDamaged) "/Game/DemonSlayer/Textures/Enemy/Demon1/Hurt/DemonHurt.DemonHurt" (select (Variables|Default|GetbisFiring) "/Game/DemonSlayer/Textures/Enemy/Demon1/Attack/DemonAttack_1.DemonAttack_1" (select (> (Math|Vector|VectorLength (Transformation|GetVelocity)) 0.0) "/Game/DemonSlayer/Textures/Enemy/Demon1/walk/DemonWalk.DemonWalk" "/Game/DemonSlayer/Textures/Enemy/Demon1/Idle/DemonIdle.DemonIdle"))))))

(event Custom|FireStop
  ;[1 1 1] Handle Fire
  (Utilities|FlowControl|Delay 0.0)
  (Variables|Default|SetbisFiring false))

(event Custom|FireStart
  (bind _returnvalue (Actor|GetGameTimeSinceCreation))
  (bind _player (Variables|Default|GetPlayer))
  ;[1 1 1] Handle Fire
  (if (>= (- _returnvalue (Variables|Default|GetlastFireTime)) (Variables|Default|GetfireRate))
    (Variables|Default|SetbisFiring true)
    (Variables|Default|SetlastFireTime _returnvalue)
    (Components|Activation|Activate (Variables|Default|GetAtack) false)
    (Utilities|FlowControl|Delay 0.3)
    (if (<= (Transformation|GetDistanceTo (Game|Player|GetPlayerPawn 0)) (Variables|Default|GetFireDist))
      (Components|Activation|Activate (Variables|/Game/DemonSlayer/Blueprints/SlayerPawn.SlayerPawn_C|GetPainSound (Variables|Default|GetPlayer)) false)
      (Variables|/Game/DemonSlayer/Blueprints/SlayerPawn.SlayerPawn_C|SetHealth _player (- (Variables|/Game/DemonSlayer/Blueprints/SlayerPawn.SlayerPawn_C|GetHealth _player) 0.1)))))

(event Custom|Move
  (params (Value :type Float%20%28single-precision%29))
  ;[1 1 1] Handle movement
  (if (> Value 0.0)
    (Variables|Default|SetbisMovingRight true)
    (elif (< Value 0.0)
      (Variables|Default|SetbisMovingRight false)))
  (Pawn|Input|AddMovementInput "1.000000, 0, 0" Value false))

(event Custom|UpdateTarget
  (bind _returnvalue (Game|Player|GetPlayerPawn 0))
  (if (<= (Transformation|GetDistanceTo _returnvalue) (Variables|Default|GetfollowDist))
    (Variables|Default|SetCurrentTarget (Transformation|GetActorTransform _returnvalue) :!label _label)
    (elif (> (Utilities|Array|Length (Variables|Default|GetTargets)) 0)
      (Variables|Default|SetCurrentTarget (Transformation|GetActorTransform (Utilities|Array|Get(acopy) (Variables|Default|GetTargets) (Variables|Default|GetTargetIndex))))
      (if (Math|Float|NearlyEqual(Float) (.x (.location (Transformation|GetActorTransform))) (.x (.location (Variables|Default|GetCurrentTarget))) (Variables|Default|Gettolerence))
        (if (< (Variables|Default|GetTargetIndex) (- (Utilities|Array|Length (Variables|Default|GetTargets)) 1))
          (bind _output_get (Variables|Default|SetTargetIndex (+ (Variables|Default|GetTargetIndex) 1)))
          (Variables|Default|SetCurrentTarget (Transformation|GetActorTransform (Utilities|Array|Get(acopy) (Variables|Default|GetTargets) _output_get)))
          (else
            (bind _output_get_2 (Variables|Default|SetTargetIndex 0))
            (Variables|Default|SetCurrentTarget (Transformation|GetActorTransform (Utilities|Array|Get(acopy) (Variables|Default|GetTargets) _output_get_2))))))
      (else
        (goto _label)))))

(event Custom|UpdateMovement
  (bind _returnvalue (Transformation|GetActorTransform))
  (bind _currenttarget (Variables|Default|GetCurrentTarget))
  (bind _tolerence (Variables|Default|Gettolerence))
  (bind _returnvalue_2 (- (.location _currenttarget) (.location _returnvalue)))
  (bind _x (Math|Vector|BreakVector _returnvalue_2))
  (if (not (Variables|Default|GetbisDead))
    (if (> _x _tolerence)
      (CallFunction|Move 1.0)
      (elif (< _x (* _tolerence -1.0))
        (CallFunction|Move -1.0)))))

(event Custom|Update%20Fire
  (bind _charactermovement (Variables|Character|GetCharacterMovement))
  (if (not (Variables|Default|GetbisDamaged))
    (if (<= (Transformation|GetDistanceTo (Game|Player|GetPlayerPawn 0)) (Variables|Default|GetFireDist))
      (Variables|/Script/Engine.CharacterMovementComponent|SetMaxWalkSpeed _charactermovement 0.0)
      (CallFunction|FireStart)
      (else
        (Variables|/Script/Engine.CharacterMovementComponent|SetMaxWalkSpeed _charactermovement (Variables|Default|GetSpeed))
        (CallFunction|FireStop)))))

(event Collision|EventActorBeginOverlap
  (params (OtherActor :type Actor%20Object%20Reference))
  (if (Variables|Default|GetbisSpawned)
    (if (== (Utilities|GetClass OtherActor) "/Game/DemonSlayer/Blueprints/Bullet.Bullet_C")
      (Variables|Default|SetHealth (- (Variables|Default|GetHealth) 0.25))
      (if (<= (Variables|Default|GetHealth) 0.0)
        (Variables|Default|SetbisDead true)
        (Collision|SetCollisionEnabled (Variables|Collision|GetCapsuleComponent) "NoCollision")
        (bind _returnvalue (Game|SpawnActorfromClass "/Game/DemonSlayer/Blueprints/HealthPickUP.HealthPickUP_C" (Math|Transform|MakeTransform (.location (Transformation|GetWorldTransform (Variables|Default|GetArrow1))) "0, 0, 0" "0.065000,0.065000,0.065000") "AdjustIfPossibleButAlwaysSpawn" 0 0))
        (Math|Float|CompareFloat (.x (- (Transformation|GetActorLocation (Game|Player|GetPlayerPawn 0)) (Transformation|GetActorLocation))) 0.0
          (:>
            (Variables|Default|SetpickUPVel "500.000000, 0,200.000000"))
          (:==
            (Variables|Default|SetpickUPVel "0, 0,200.000000"))
          (:<
            (Variables|Default|SetpickUPVel "-500.000000, 0,200.000000")))
        (Physics|SetPhysicsLinearVelocity (Variables|/Game/DemonSlayer/Blueprints/HealthPickUP.HealthPickUP_C|GetPaperSprite _returnvalue) (Variables|Default|GetpickUPVel) true "None")
        (Pawn|Components|CharacterMovement|DisableMovement (Variables|Character|GetCharacterMovement))
        (Utilities|FlowControl|Delay 0.85)
        (Actor|DestroyActor)
        (else
          (Variables|Default|SetbisDamaged true)
          (Utilities|FlowControl|Delay 0.55)
          (Variables|Default|SetbisDamaged false))))))

(event EventTick
  (params (DeltaSeconds :type Float%20%28single-precision%29))
  ;[1 1 1] Tick - Updates animation
  (if (Variables|Default|GetbisSpawned)
    (CallFunction|UpdateAnimation)
    (CallFunction|UpdateTarget)
    (CallFunction|UpdateMovement)
    (CallFunction|UpdateFire)
    (Math|Float|CompareFloat (.X (Math|Vector|BreakVector (- (.location (Variables|Default|GetCurrentTarget)) (.location (Transformation|GetActorTransform))))) 0.0
      (:>
        (Transformation|SetRelativeRotation (Variables|Default|GetSprite) (Math|Rotator|MakeRotator 0.0 0.0 0.0) false false))
      (:<
        (Transformation|SetRelativeRotation (Variables|Default|GetSprite) (Math|Rotator|MakeRotator 0.0 0.0 1.8e+02) false false)))
    (elif (Variables|Default|GetbisShoudSpawn)
      (CallFunction|Spawn))))

(event EventBeginPlay
  (bind _targets (Variables|Default|GetTargets))
  (Class|ActorComponent|SetIsReplicated (Variables|Default|GetSprite) true)
  (bind _asslayer_pawn (Utilities|Casting|CastToSlayerPawn (Game|Player|GetPlayerPawn 0)))
  (Variables|Default|SetPlayer _asslayer_pawn)
  (if (> (Utilities|Array|Length _targets) 0)
    (if (> (Utilities|Array|Length _targets) 0)
      (Variables|Default|SetCurrentTarget (Transformation|GetActorTransform (Utilities|Array|Get(acopy) _targets)))
      (Variables|Default|SetSpeed (Class|MovementComponent|GetMaxSpeed (Variables|Character|GetCharacterMovement)) :!label _label))
    (else
      (goto _label))))

(fn ConstructionScript)