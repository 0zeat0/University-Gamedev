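; Level exit door that loads another level by name when the SlayerPawn uses it after it has been opened.
; Overlap toggles the text prompt and registers or clears the door as the player's UseObject.
; The Open event unlocks the door and changes the prompt to a key hint.
; Use then swaps to the open sprite, disables overlaps and loads the level after a short delay.
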(event Custom|Use
  (if (Variables|Default|GetbOpen)
    (if (Variables|Default|GetbCanUse)
      (Rendering|Components|Sprite|SetSprite (Variables|Default|Getdoor_Sprite) "/Game/DemonSlayer/Sprites/Level/dooropen_Sprite.dooropen_Sprite")
      (Rendering|SetVisibility (Variables|Default|GetTextRender) false false)
      (Variables|Default|SetbCanUse false)
      (Variables|/Script/Engine.PrimitiveComponent|SetbGenerateOverlapEvents (Variables|Default|Getdoor_Sprite) false)
      (Utilities|FlowControl|Delay 1.0)
      (Game|OpenLevel(byName) (Variables|Default|GetLevel)))))

(event Custom|Open
  (Rendering|Components|TextRender|SetText (Variables|Default|GetTextRender) (Utilities|Text|FormatText "Press E"))
  (Variables|Default|SetbOpen true))

(event Collision|EventActorBeginOverlap
  (params (OtherActor :type Actor%20Object%20Reference))
  (if (== (Utilities|GetClass OtherActor) "/Game/DemonSlayer/Blueprints/SlayerPawn.SlayerPawn_C")
    (Rendering|SetVisibility (Variables|Default|GetTextRender) true false)
    (Variables|Default|SetbCanUse true)
    (Variables|/Game/DemonSlayer/Blueprints/SlayerPawn.SlayerPawn_C|SetUseObject (Variables|Default|GetPlayer) self)))

(event Collision|EventActorEndOverlap
  (params (OtherActor :type Actor%20Object%20Reference))
  (if (== (Utilities|GetClass OtherActor) "/Game/DemonSlayer/Blueprints/SlayerPawn.SlayerPawn_C")
    (Rendering|SetVisibility (Variables|Default|GetTextRender) false false)
    (Variables|Default|SetbCanUse false)
    (Variables|/Game/DemonSlayer/Blueprints/SlayerPawn.SlayerPawn_C|SetUseObject (Variables|Default|GetPlayer) 0)))

(event EventBeginPlay
  (bind _asslayer_pawn (Utilities|Casting|CastToSlayerPawn (Game|Player|GetPlayerPawn 0)))
  (Variables|Default|SetPlayer _asslayer_pawn))

(fn ConstructionScript)