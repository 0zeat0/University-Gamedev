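; Health pickup for the 2D Demon Slayer game that is drawn toward a hurt player.
; While the SlayerPawn's health is below 1.0 and within range, Tick adds fixed velocity steps to the physics-driven sprite along X and Z toward the pawn, easing velocity toward zero on exact alignment.
; Overlapping the pawn while it is hurt calls its PickUPEvent and destroys the pickup.
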(event EventBeginPlay
  (bind _asslayer_pawn (Utilities|Casting|CastToSlayerPawn (Game|Player|GetPlayerPawn 0)))
  (Variables|Default|SetPlayer _asslayer_pawn))

(event Collision|EventActorBeginOverlap
  (params (OtherActor :type Actor%20Object%20Reference))
  (if (== (Utilities|GetClass OtherActor) "/Game/DemonSlayer/Blueprints/SlayerPawn.SlayerPawn_C")
    (if (< (Variables|/Game/DemonSlayer/Blueprints/SlayerPawn.SlayerPawn_C|GetHealth (Variables|Default|GetPlayer)) 1.0)
      (Default|PickUPEvent (Variables|Default|GetPlayer))
      (Actor|DestroyActor))))

(event EventTick
  (params (DeltaSeconds :type Float%20%28single-precision%29))
  (bind _returnvalue (Game|Player|GetPlayerPawn 0))
  (bind _returnvalue_2 (Transformation|GetActorTransform))
  (bind _papersprite (Variables|Default|GetPaperSprite))
  (bind _returnvalue_3 (Transformation|GetActorTransform _returnvalue))
  (bind _returnvalue_4 (- (.location _returnvalue_2) (.location _returnvalue_3)))
  (if (< (Variables|/Game/DemonSlayer/Blueprints/SlayerPawn.SlayerPawn_C|GetHealth (Variables|Default|GetPlayer)) 1.0)
    (if (<= (Transformation|GetDistanceTo (Game|Player|GetPlayerPawn 0)) 4e+02)
      (Math|Float|CompareFloat (.x _returnvalue_4) 0.0
        (:>
          (Physics|SetPhysicsLinearVelocity _papersprite "-10.000000, 0, 0" true "None")
          (Math|Float|CompareFloat (.z _returnvalue_4) 0.0 :!label _label
            (:>
              (Physics|SetPhysicsLinearVelocity _papersprite "-0.000000, 0,-10.000000" true "None"))
            (:==
              (Physics|SetPhysicsLinearVelocity (Variables|Default|GetPaperSprite) (Math|Interpolation|VInterpTo (Transformation|GetVelocity) "0, 0, 0" 0.0 5.0) false "None" :!label _label_2))
            (:<
              (Physics|SetPhysicsLinearVelocity _papersprite "0.000000, 0,10.000000" true "None"))))
        (:==
          (goto _label_2))
        (:<
          (Physics|SetPhysicsLinearVelocity _papersprite "10.000000, 0, 0" true "None")
          (goto _label))))))

(fn ConstructionScript)