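; Interactable computer terminal for DemonSlayer that the player uses to open linked doors and optionally spawn demons.
; Overlap with SlayerPawn shows a text prompt and registers the terminal as the player's use object; leaving clears both.
; Using it swaps the sprite, hides the prompt and disables further use.
; It then calls the spawn function on listed EnemyDemons if enabled, and opens every door in its array.
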(event Custom|Use
  (if (Variables|Default|GetbCanUse)
    (Rendering|Components|Sprite|SetSprite (Variables|Default|GetPaperSprite) "/Game/DemonSlayer/Sprites/Level/comp_Sprite.comp_Sprite")
    (Rendering|SetVisibility (Variables|Default|GetTextRender) false false)
    (Variables|Default|SetbCanUse false)
    (Variables|/Script/Engine.PrimitiveComponent|SetbGenerateOverlapEvents (Variables|Default|GetPaperSprite) false)
    (if (Variables|Default|GetbSpawnEnemys)
      (for _array_element (Variables|Default|GetEnemys)
        (if (== (Utilities|GetClass _array_element) "/Game/DemonSlayer/Blueprints/EnemyDemon.EnemyDemon_C")
          (bind _asenemy_demon (Utilities|Casting|CastToEnemyDemon _array_element))
          (Default|ShoudSpaawn _asenemy_demon))))
    (for _array_element_2 (Variables|Default|GetDoors)
      (Default|Open _array_element_2))))

(event Collision|EventActorBeginOverlap
  (params (OtherActor :type Actor%20Object%20Reference))
  (if (== (Utilities|GetClass OtherActor) "/Game/DemonSlayer/Blueprints/SlayerPawn.SlayerPawn_C")
    (Rendering|SetVisibility (Variables|Default|GetTextRender) true false)
    (Variables|Default|SetbCanUse true)
    (Variables|/Game/DemonSlayer/Blueprints/SlayerPawn.SlayerPawn_C|SetUseObject (Variables|Default|GetPlayer) self)))

(event Collision|EventActorEndOverlap
  (params (OtherActor :type Actor%20Object%20Reference))
  (if (== (Utilities|GetClass OtherActor) "/Game/DemonSlayer/Blueprints/SlayerPawn.SlayerPawn_C")
    (Rendering|SetVisibility (Variables|Default|GetTextRender) false false)
    (Variables|Default|SetbCanUse false)
    (Variables|/Game/DemonSlayer/Blueprints/SlayerPawn.SlayerPawn_C|SetUseObject (Variables|Default|GetPlayer) 0)))

(event EventBeginPlay
  (bind _asslayer_pawn (Utilities|Casting|CastToSlayerPawn (Game|Player|GetPlayerPawn 0)))
  (Variables|Default|SetPlayer _asslayer_pawn))

(fn ConstructionScript)