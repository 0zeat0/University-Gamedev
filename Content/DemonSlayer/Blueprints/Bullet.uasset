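; Bullet is a physics-driven projectile actor that launches along the SlayerPawn's facing direction and explodes on EnemyDemon contact.
; On BeginPlay it flips its velocity if the pawn faces left, applies it with random per-axis recoil spread, and expires after five seconds.
; Other surfaces allow a limited number of hits before detonation.
; Detonation swaps the bullet for explosion visuals, stops physics motion, flares two lights, plays sound, then destroys the actor.
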(event EventBeginPlay
  (bind _minrecoil (Variables|Default|GetminRecoil))
  (bind _maxrecoil (Variables|Default|GetmaxRecoil))
  (bind _asslayer_pawn (Utilities|Casting|CastToSlayerPawn (Game|Player|GetPlayerPawn 0)))
  (Variables|Default|SetPlayerPawn _asslayer_pawn)
  (if (Variables|/Game/DemonSlayer/Blueprints/SlayerPawn.SlayerPawn_C|GetbisMovingRight (Variables|Default|GetPlayerPawn))
    _
    (else
      (Variables|Default|SetVelocity (* (Variables|Default|GetVelocity) -1.0))))
  (Physics|SetPhysicsLinearVelocity (Variables|Default|GetSphere1) (+ (Variables|Default|GetVelocity) (Math|Vector|MakeVector (+ (.X (Math|Vector|BreakVector (Variables|Default|GetVelocity))) (Math|Random|RandomFloatinRange _minrecoil _maxrecoil)) (+ (.Y (Math|Vector|BreakVector (Variables|Default|GetVelocity))) (Math|Random|RandomFloatinRange _minrecoil _maxrecoil)) (+ (.Z (Math|Vector|BreakVector (Variables|Default|GetVelocity))) (Math|Random|RandomFloatinRange _minrecoil _maxrecoil)))) true "None")
  (Utilities|FlowControl|Delay 5.0)
  (Actor|DestroyActor))

(event Collision|EventActorBeginOverlap
  (params (OtherActor :type Actor%20Object%20Reference))
  (bind _sphere1 (Variables|Default|GetSphere1))
  (bind _light (Variables|Default|Getlight))
  (bind _light1 (Variables|Default|Getlight1))
  (if (== (Utilities|GetClass OtherActor) "/Game/DemonSlayer/Blueprints/EnemyDemon.EnemyDemon_C")
    (Rendering|SetVisibility (Variables|Default|GetBullet) false false)
    (Rendering|SetVisibility (Variables|Default|GetExp) true false)
    (Physics|SetPhysicsLinearVelocity _sphere1 "0, 0, 0" false "None")
    (Physics|SetEnableGravity _sphere1 false)
    (Rendering|Lighting|SetAttenuationRadius _light 5e+02)
    (Rendering|Lighting|SetAttenuationRadius _light1 5e+02)
    (Rendering|Components|Light|SetIntensity _light 8e+03)
    (Rendering|Components|Light|SetIntensity _light1 8e+03)
    (Components|Activation|Activate (Variables|Default|GetExpSound) false)
    (Utilities|FlowControl|Delay 0.85)
    (Actor|DestroyActor)))

(event Collision|EventHit
  (params (MyComp :type Primitive%20Component%20Object%20Reference) (Other :type Actor%20Object%20Reference) (OtherComp :type Primitive%20Component%20Object%20Reference) (bSelfMoved :type Boolean) (HitLocation :type Vector :default "0, 0, 0") (HitNormal :type Vector :default "0, 0, 0") (NormalImpulse :type Vector :default "0, 0, 0") (Hit :type Hit%20Result%20Structure%20%28by%20ref%29))
  (bind _sphere1 (Variables|Default|GetSphere1))
  (bind _light (Variables|Default|Getlight))
  (bind _light1 (Variables|Default|Getlight1))
  (if (== (Utilities|GetClass Other) "/Game/DemonSlayer/Blueprints/EnemyDemon.EnemyDemon_C")
    (Rendering|SetVisibility (Variables|Default|GetBullet) false false :!label _label)
    (Rendering|SetVisibility (Variables|Default|GetExp) true false)
    (Physics|SetPhysicsLinearVelocity _sphere1 "0, 0, 0" false "None")
    (Physics|SetEnableGravity _sphere1 false)
    (Rendering|Lighting|SetAttenuationRadius _light 5e+02)
    (Rendering|Lighting|SetAttenuationRadius _light1 5e+02)
    (Rendering|Components|Light|SetIntensity _light 8e+03)
    (Rendering|Components|Light|SetIntensity _light1 8e+03)
    (Components|Activation|Activate (Variables|Default|GetExpSound) false)
    (Utilities|FlowControl|Delay 0.85)
    (Actor|DestroyActor)
    (elif (< (Variables|Default|GethitCount) (Variables|Default|GetmaxHitCount))
      (Variables|Default|SethitCount (+ (Variables|Default|GethitCount) 1))
      (else
        (goto _label)))))

(fn ConstructionScript)