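; Trap is a one-shot spawn trigger that releases preset demons when the Slayer player overlaps it.
; On overlap by a SlayerPawn, it loops through its Enemy array and calls the spawn function on each EnemyDemon or FlyDemon entry.
; An activation flag set during the loop keeps the trap from firing again.
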(event Collision|EventActorBeginOverlap
  (params (OtherActor :type Actor%20Object%20Reference))
  (if (not (Variables|Default|GetbisActivated))
    (if (== (Utilities|GetClass OtherActor) "/Game/DemonSlayer/Blueprints/SlayerPawn.SlayerPawn_C")
      (for _array_element (Variables|Default|GetEnemy)
        (if (== (Utilities|GetClass _array_element) "/Game/DemonSlayer/Blueprints/EnemyDemon.EnemyDemon_C")
          (bind _asenemy_demon (Utilities|Casting|CastToEnemyDemon _array_element))
          (Default|ShoudSpaawn _asenemy_demon)
          (Variables|Default|SetbisActivated true)
          (elif (== (Utilities|GetClass _array_element) "/Game/DemonSlayer/Blueprints/FlyDemon.FlyDemon_C")
            (bind _asfly_demon (Utilities|Casting|CastToFlyDemon _array_element))
            (Default|ShoudSpaawn _asfly_demon)
            (Variables|Default|SetbisActivated true)))))))

(fn ConstructionScript)