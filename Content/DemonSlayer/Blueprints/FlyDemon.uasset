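; Flying demon enemy for a Paper2D side-scroller that patrols target points and attacks the player with fireballs.
; It stays dormant until flagged and within spawn distance, then appears with particles and sound.
; Tick drives flipbook choice, facing, X/Z steering between waypoints, and stop-to-fire when the player is in range, with rate-limited, delayed shots.
; Bullet overlaps cause damage that pauses attack checks; death launches a health pickup toward the player before destruction.
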(event Custom|Spawn
  (if (<= (Transformation|GetDistanceTo (Game|Player|GetPlayerPawn 0)) (Variables|Default|GetSpawnDistance))
    (Utilities|FlowControl|DoOnce false
      (:Completed
        (Components|Activation|Activate (Variables|Default|GetParticleSystem) false)
        (Utilities|FlowControl|Delay 2.0)
        (Components|Activation|Activate (Variables|Default|GetSpawnAudio) false)
        (Rendering|SetVisibility (Variables|Default|GetSprite) true false)
        (Utilities|FlowControl|Delay 1.6)
        (Components|DestroyComponent (Variables|Default|GetParticleSystem))
        (Variables|Default|SetbisSpawned true)
        (Components|Activation|Activate (Variables|Default|GetMonster) false)
        (Variables|/Script/Engine.PrimitiveComponent|SetbGenerateOverlapEvents (Variables|Collision|GetCapsuleComponent) true)))))

(event Custom|ShoudSpaawn
  (Variables|Default|SetSpawnDistance 1e+05)
  (Variables|Default|SetbisShoudSpawn true))

(event Custom|UpdateAnimation
  ;[1 1 1] Handle Animation
  (Sprite|SetFlipbook (Variables|Default|GetSprite) (select (Variables|Default|GetbisDead) "/Game/DemonSlayer/Textures/FlyDemon/Death/Death.Death" (select (Variables|Default|GetbisFiring) "/Game/DemonSlayer/Textures/FlyDemon/Atack/Attack.Attack" (select (> (Math|Vector|VectorLength (Transformation|GetVelocity)) 0.0) "/Game/DemonSlayer/Textures/FlyDemon/Idle/Idle.Idle" "/Game/DemonSlayer/Textures/FlyDemon/Idle/Idle.Idle")))))

(event Custom|FireStop
  ;[1 1 1] Handle Fire
  (Utilities|FlowControl|Delay 0.0)
  (Variables|Default|SetbisFiring false))

(event Custom|FireStart
  (bind _returnvalue (Actor|GetGameTimeSinceCreation))
  ;[1 1 1] Handle Fire
  (if (>= (- _returnvalue (Variables|Default|GetlastFireTime)) (Variables|Default|GetfireRate))
    (Variables|Default|SetbisFiring true)
    (Variables|Default|SetlastFireTime _returnvalue)
    (Components|Activation|Activate (Variables|Default|GetAtack) false)
    (Utilities|FlowControl|Delay 0.3)
    (if (<= (Transformation|GetDistanceTo (Game|Player|GetPlayerPawn 0)) (Variables|Default|GetFireDist))
      (Components|Activation|Activate (Variables|/Game/DemonSlayer/Blueprints/SlayerPawn.SlayerPawn_C|GetPainSound (Variables|Default|GetPlayer)) false)
      (Game|SpawnActorfromClass "/Game/DemonSlayer/Blueprints/FireBall.FireBall_C" (Math|Transform|MakeTransform (.location (Transformation|GetWorldTransform (Variables|Default|GetSpawnFB))) "0, 0, 0" "1,1,1") "AlwaysSpawn" 0 0))))

(event Custom|MoveRight
  (params (Value :type Float%20%28single-precision%29))
  ;[1 1 1] Handle movement
  (if (> Value 0.0)
    (Variables|Default|SetbisMovingRight true)
    (elif (< Value 0.0)
      (Variables|Default|SetbisMovingRight false)))
  (Pawn|Input|AddMovementInput "1.000000, 0, 0" Value false))

(event Custom|MoveTop
  (params (Value :type Float%20%28single-precision%29))
  ;[1 1 1] Handle movement
  (if (> Value 0.0)
    _
    (elif (< Value 0.0)
      _
      (else
        _)))
  (Pawn|Input|AddMovementInput "0.000000,0.000000,1.000000" Value false))

(event Custom|UpdateTarget
  (Variables|Default|SetCurrentTarget (Transformation|GetActorTransform (Utilities|Array|Get(acopy) (Variables|Default|GetTargets) (Variables|Default|GetTargetIndex))))
  (if (Math|Float|NearlyEqual(Float) (.x (.location (Transformation|GetActorTransform))) (.x (.location (Variables|Default|GetCurrentTarget))) (Variables|Default|Gettolerence))
    (if (< (Variables|Default|GetTargetIndex) (- (Utilities|Array|Length (Variables|Default|GetTargets)) 1))
      (bind _output_get (Variables|Default|SetTargetIndex (+ (Variables|Default|GetTargetIndex) 1)))
      (Variables|Default|SetCurrentTarget (Transformation|GetActorTransform (Utilities|Array|Get(acopy) (Variables|Default|GetTargets) _output_get)))
      (else
        (bind _output_get_2 (Variables|Default|SetTargetIndex 0))
        (Variables|Default|SetCurrentTarget (Transformation|GetActorTransform (Utilities|Array|Get(acopy) (Variables|Default|GetTargets) _output_get_2)))))))

(event Custom|UpdateMovement
  (bind _returnvalue (Transformation|GetActorTransform))
  (bind _returnvalue_2 (Transformation|GetActorTransform))
  (bind _currenttarget (Variables|Default|GetCurrentTarget))
  (bind _tolerence (Variables|Default|Gettolerence))
  (bind _currenttarget_2 (Variables|Default|GetCurrentTarget))
  (bind _tolerence_2 (Variables|Default|Gettolerence))
  (bind _returnvalue_3 (- (.location _currenttarget) (.location _returnvalue_2)))
  (bind _returnvalue_4 (- (.location _currenttarget_2) (.location _returnvalue)))
  (bind _z (Math|Vector|BreakVector _returnvalue_3))
  (bind _x (Math|Vector|BreakVector _returnvalue_4))
  (if (not (Variables|Default|GetbisDead))
    (Utilities|FlowControl|Sequence
      (:then_0
        (if (> _x _tolerence_2)
          (CallFunction|MoveRight 1.0)
          (elif (< _x (* _tolerence_2 -1.0))
            (CallFunction|MoveRight -1.0))))
      (:then_1
        (if (> _z _tolerence)
          (CallFunction|MoveTop 1.0)
          (elif (< _z (* _tolerence -1.0))
            (CallFunction|MoveTop -1.0)))))))

(event Custom|Update%20Fire
  (bind _charactermovement (Variables|Character|GetCharacterMovement))
  (if (not (Variables|Default|GetbisDamaged))
    (if (<= (Transformation|GetDistanceTo (Game|Player|GetPlayerPawn 0)) (Variables|Default|GetFireDist))
      (Components|Movement|StopMovementImmediately _charactermovement)
      (Variables|/Script/Engine.CharacterMovementComponent|SetMaxFlySpeed _charactermovement 0.0)
      (CallFunction|FireStart)
      (else
        (Variables|/Script/Engine.CharacterMovementComponent|SetMaxFlySpeed _charactermovement (Variables|Default|GetSpeed))
        (CallFunction|FireStop)))))

(event Collision|EventActorBeginOverlap
  (params (OtherActor :type Actor%20Object%20Reference))
  (if (Variables|Default|GetbisSpawned)
    (if (== (Utilities|GetClass OtherActor) "/Game/DemonSlayer/Blueprints/Bullet.Bullet_C")
      (Variables|Default|SetHealth (- (Variables|Default|GetHealth) 0.25))
      (if (<= (Variables|Default|GetHealth) 0.0)
        (Variables|Default|SetbisDead true)
        (Collision|SetCollisionEnabled (Variables|Collision|GetCapsuleComponent) "NoCollision")
        (bind _returnvalue (Game|SpawnActorfromClass "/Game/DemonSlayer/Blueprints/HealthPickUP.HealthPickUP_C" (Math|Transform|MakeTransform (.location (Transformation|GetWorldTransform (Variables|Default|GetArrow1))) "0, 0, 0" "0.065000,0.065000,0.065000") "AdjustIfPossibleButAlwaysSpawn" 0 0))
        (Math|Float|CompareFloat (.x (- (Transformation|GetActorLocation (Game|Player|GetPlayerPawn 0)) (Transformation|GetActorLocation))) 0.0
          (:>
            (Variables|Default|SetpickUPVel "500.000000, 0,200.000000"))
          (:==
            (Variables|Default|SetpickUPVel "0, 0,200.000000"))
          (:<
            (Variables|Default|SetpickUPVel "-500.000000, 0,200.000000")))
        (Physics|SetPhysicsLinearVelocity (Variables|/Game/DemonSlayer/Blueprints/HealthPickUP.HealthPickUP_C|GetPaperSprite _returnvalue) (Variables|Default|GetpickUPVel) true "None")
        (Pawn|Components|CharacterMovement|DisableMovement (Variables|Character|GetCharacterMovement))
        (Utilities|FlowControl|Delay 0.85)
        (Actor|DestroyActor)
        (else
          (Variables|Default|SetbisDamaged true)
          (Utilities|FlowControl|Delay 0.55)
          (Variables|Default|SetbisDamaged false))))))

(event EventTick
  (params (DeltaSeconds :type Float%20%28single-precision%29))
  ;[1 1 1] Tick - Updates animation
  (if (Variables|Default|GetbisSpawned)
    (CallFunction|UpdateAnimation)
    (CallFunction|UpdateTarget)
    (CallFunction|UpdateMovement)
    (CallFunction|UpdateFire)
    (if (not (Variables|Default|GetbisFiring))
      (Math|Float|CompareFloat (.X (Math|Vector|BreakVector (- (.location (Variables|Default|GetCurrentTarget)) (.location (Transformation|GetActorTransform))))) 0.0
        (:>
          (Transformation|SetRelativeRotation (Variables|Default|GetSprite) (Math|Rotator|MakeRotator 0.0 0.0 0.0) false false))
        (:<
          (Transformation|SetRelativeRotation (Variables|Default|GetSprite) (Math|Rotator|MakeRotator 0.0 0.0 1.8e+02) false false)))
      (else
        (Math|Float|CompareFloat (.X (Math|Vector|BreakVector (- (Transformation|GetActorLocation (Game|Player|GetPlayerPawn 0)) (.location (Transformation|GetActorTransform))))) 0.0
          (:>
            (Transformation|SetRelativeRotation (Variables|Default|GetSprite) (Math|Rotator|MakeRotator 0.0 0.0 0.0) false false))
          (:<
            (Transformation|SetRelativeRotation (Variables|Default|GetSprite) (Math|Rotator|MakeRotator 0.0 0.0 1.8e+02) false false)))))
    (elif (Variables|Default|GetbisShoudSpawn)
      (CallFunction|Spawn))))

(event EventBeginPlay
  (bind _targets (Variables|Default|GetTargets))
  (Class|ActorComponent|SetIsReplicated (Variables|Default|GetSprite) true)
  (bind _asslayer_pawn (Utilities|Casting|CastToSlayerPawn (Game|Player|GetPlayerPawn 0)))
  (Variables|Default|SetPlayer _asslayer_pawn)
  (if (> (Utilities|Array|Length _targets) 0)
    (if (> (Utilities|Array|Length _targets) 0)
      (Variables|Default|SetCurrentTarget (Transformation|GetActorTransform (Utilities|Array|Get(acopy) _targets)))
      (Variables|Default|SetSpeed (Variables|/Script/Engine.CharacterMovementComponent|GetMaxFlySpeed (Variables|Character|GetCharacterMovement)) :!label _label))
    (else
      (goto _label))))

(fn ConstructionScript)